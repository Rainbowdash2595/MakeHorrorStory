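; Interactable bed that lets the first-person character hide and come back out with the Interacting input.
; A Box overlap stores the character, enables input and opens a Gate; leaving disables input and closes it.
; ToggleHide flips the character's visibility and collision, blending the view between bed and character.
; A short delay after each toggle re-enables input and reopens the Gate, even if the overlap has ended.
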(event OnComponentBeginOverlap(Box)
  (params (OverlappedComponent :type Primitive%20Component%20Object%20Reference) (OtherActor :type Actor%20Object%20Reference) (OtherComp :type Primitive%20Component%20Object%20Reference) (OtherBodyIndex :type Integer) (bFromSweep :type Boolean) (SweepResult :type Hit%20Result%20Structure%20%28by%20ref%29))
  (bind _asfirst_person_character_bp (Utilities|Casting|CastToFirstPersonCharacter_BP OtherActor))
  (Variables|Default|SetCharRef _asfirst_person_character_bp)
  (Input|EnableInput (Game|GetPlayerController 0))
  (Utilities|FlowControl|Gate true) ; enters at Open
)

(event OnComponentEndOverlap(Box)
  (params (OverlappedComponent :type Primitive%20Component%20Object%20Reference) (OtherActor :type Actor%20Object%20Reference) (OtherComp :type Primitive%20Component%20Object%20Reference) (OtherBodyIndex :type Integer))
  (bind _returnvalue (Game|GetPlayerController 0))
  (Utilities|Casting|CastToFirstPersonCharacter_BP OtherActor)
  (Input|DisableInput _returnvalue)
  (Utilities|FlowControl|Gate true) ; enters at Close
)

(event Input|ActionEvents|InputActionInteracting
  (params (Key :type Key%20Structure :default "None"))
  (:Pressed
    (Utilities|FlowControl|Gate true :!label _label
      (:Exit
        (CallFunction|ToggleHide)
        (Utilities|FlowControl|Delay 0.2)
        (Input|EnableInput (Game|GetPlayerController 0))
        (goto _label Open)))))

(fn ConstructionScript)

(fn ToggleHide
  (bind _returnvalue (Game|GetPlayerController 0))
  (bind _charref (Variables|Default|GetCharRef))
  (if (Variables|Default|GetIsHide?)
    (Variables|Default|SetIsHide? false)
    (Rendering|SetActorHiddenInGame _charref false)
    (Collision|SetActorEnableCollision _charref true)
    (Game|Player|SetViewTargetwithBlend _returnvalue _charref 0.6 "VTBlend_Linear" 0.0 false)
    (else
      (Variables|Default|SetIsHide? true)
      (Rendering|SetActorHiddenInGame _charref true)
      (Collision|SetActorEnableCollision _charref false)
      (Game|Player|SetViewTargetwithBlend _returnvalue self 0.6 "VTBlend_Linear" 0.0 false))))